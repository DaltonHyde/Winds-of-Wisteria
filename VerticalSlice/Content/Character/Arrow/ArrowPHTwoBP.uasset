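; ArrowPHTwoBP is an arrow actor in the character's arrow set that tilts to follow its flight path.
; On BeginPlay it sets its actor tags to PlayerWeaponTag, marking it as a player weapon.
; Every Tick calls ArrowAngleTwo, which takes the pitch from the velocity vector and applies it to the actor while keeping its current roll and yaw.
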(event `self.ReceiveBeginPlay`
  (set `self.Tags` (`|MakeArray` (`self.PlayerWeaponTag`))))

(event `self.ReceiveTick`
  (params (DeltaSeconds :type "Float (single-precision)"))
  (`self.ArrowAngleTwo`)
  (if true
    _))

(event `ArrowAngleTwo`
  (`self.K2_SetActorRotation` (`KismetMathLibrary.MakeRotator` (.roll (`self.K2_GetActorRotation`)) (.pitch (`KismetMathLibrary.MakeRotFromX` (`self.GetVelocity`))) (.yaw (`self.K2_GetActorRotation`)))))

(fn `UserConstructionScript`)