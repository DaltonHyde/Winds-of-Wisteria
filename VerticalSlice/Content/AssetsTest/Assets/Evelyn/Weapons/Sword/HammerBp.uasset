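; HammerBp is a player weapon actor that damages enemies it overlaps and tags itself as a player weapon on BeginPlay.
; On overlap, it checks that the other actor has a skeletal mesh with the Enemy collision object type, then applies its hammer damage.
; A HitEnemy flag with a short delayed reset blocks repeated hits from one swing.
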(event `self.ReceiveBeginPlay`
  (set `self.Tags` (`|MakeArray` (`self.PlayerWeaponTag`))))

(event `self.ReceiveActorBeginOverlap`
  (params (OtherActor :type "Actor Object Reference"))
  (bind _returnvalue (`self.GetComponentByClass` OtherActor "/Script/Engine.SkeletalMeshComponent"))
  (if (`self.HitEnemy`)
    _
    (elif (`KismetSystemLibrary.IsValid` _returnvalue)
      (switch `ECollisionChannel` (`PrimitiveComponent.GetCollisionObjectType` _returnvalue)
        (:`ECC_GameTraceChannel3`
          (`GameplayStatics.ApplyDamage` OtherActor (`KismetMathLibrary.Conv_IntToDouble` (`self.HammerDamage`)))
          (set `self.HitEnemy` true)
          (`self.DamageDelay`))))))

(event `DamageDelay`
  (`KismetSystemLibrary.Delay` 0.3)
  (set `self.HitEnemy` false))

(fn `UserConstructionScript`)