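; Melee enemy character Blueprint that reacts when PawnSensing spots the player character.
; On sight it stores the player, sets the engagement phase, shows an exclamation text and toggles a jump-back flag between timed pauses.
; It then clears the text and calls AIMoveTo without a target actor or destination set.
; Jump-back movement, roaming and behavior tree setup sit in disconnected nodes, and Tick does nothing.
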(event `self.ReceiveBeginPlay`)

(event `self.PawnSensing.OnSeePawn`
  (params (Pawn :type "Pawn Object Reference"))
  (bind _asmy_pocchar (cast `/Game/Character/MyPOCChar` Pawn))
  (set `self.ThePlayersCharacter` _asmy_pocchar)
  (set `self.PlayerEngagementPhase` 1)
  (set `self.JumpingBack` true)
  (`TextRenderComponent.K2_SetText` (`self.Surprise`) (`self.ExclamationPoint`))
  (`KismetSystemLibrary.Delay` (`self.JumpBackPause`))
  (set `self.JumpingBack` false)
  (`KismetSystemLibrary.Delay` (`self.AfterJumpBackPause`))
  (`TextRenderComponent.K2_SetText` (`self.Surprise`) (`self.BlankSpace`))
  (`|AIMoveTo` self (0.0 0.0 0.0) null 350.0))

(event `self.ReceiveTick`
  (params (DeltaSeconds :type "Float (single-precision)"))
  (if (== (`self.PlayerEngagementPhase`) 0)
    _))

(fn `UserConstructionScript`)