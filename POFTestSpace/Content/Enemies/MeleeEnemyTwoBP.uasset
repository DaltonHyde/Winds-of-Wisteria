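; Melee enemy that detects the player, reacts with surprise on first sighting, trades damage and destroys itself after death.
; Pawn sensing sets an integer EngagementPhase through a DoOnce that resets during disengage; Tick derives the jump-back flag and exclamation text from it.
; Mesh overlaps with weapon-tagged actors reduce enemy health, while Sphere overlaps damage the player unless invulnerable.
; Tick also handles delayed destruction at zero health; arrow-damage logic remains disconnected.
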(event OnSeePawn(PawnSensing)
  (params (Pawn :type Pawn%20Object%20Reference))
  (bind _asmy_pocchar (Utilities|Casting|CastToMyPOCChar Pawn))
  (Variables|Default|SetThePlayersChar _asmy_pocchar)
  (if (!= (Variables|Default|GetEngagementPhase) (Variables|Default|GetDisengagePhase))
    (Utilities|FlowControl|DoOnce false :!label _label
      (:Completed
        (if (Variables|Default|GetFirstEncounter)
          (Variables|Default|SetFirstEncounter false)
          (Variables|Default|SetEngagementPhase 1)
          (else
            (Variables|Default|SetEngagementPhase 3)))))
    (else
      (goto _label Reset))))

(event OnComponentBeginOverlap(Mesh)
  (params (OverlappedComponent :type Primitive%20Component%20Object%20Reference) (OtherActor :type Actor%20Object%20Reference) (OtherComp :type Primitive%20Component%20Object%20Reference) (OtherBodyIndex :type Integer) (bFromSweep :type Boolean) (SweepResult :type Hit%20Result%20Structure%20%28by%20ref%29))
  (if (Actor|ActorHasTag OtherActor (Variables|Default|GetPlayerWeaponTag))
    (bind _output_get (Variables|Default|SetEnemyHealth (- (Variables|Default|GetEnemyHealth) (Variables|Default|GetDamageTaken))))
    (Development|PrintString (Utilities|String|ToString(Integer) _output_get) true true "(R=0.999713,G=0.061979,B=1.000000,A=1.000000)" 5.0)))

(event OnComponentHit(Mesh)
  (params (HitComponent :type Primitive%20Component%20Object%20Reference) (OtherActor :type Actor%20Object%20Reference) (OtherComp :type Primitive%20Component%20Object%20Reference) (NormalImpulse :type Vector :default "0, 0, 0") (Hit :type Hit%20Result%20Structure%20%28by%20ref%29)))

(event OnComponentHit(Sphere)
  (params (HitComponent :type Primitive%20Component%20Object%20Reference) (OtherActor :type Actor%20Object%20Reference) (OtherComp :type Primitive%20Component%20Object%20Reference) (NormalImpulse :type Vector :default "0, 0, 0") (Hit :type Hit%20Result%20Structure%20%28by%20ref%29))
  ;[1 1 1] Hitting Player
)

(event OnComponentBeginOverlap(Sphere)
  (params (OverlappedComponent :type Primitive%20Component%20Object%20Reference) (OtherActor :type Actor%20Object%20Reference) (OtherComp :type Primitive%20Component%20Object%20Reference) (OtherBodyIndex :type Integer) (bFromSweep :type Boolean) (SweepResult :type Hit%20Result%20Structure%20%28by%20ref%29))
  ;[1 1 1] Hitting Player
  (bind _asmy_pocchar (Utilities|Casting|CastToMyPOCChar (Game|GetPlayerCharacter 0)))
  (if (== OtherActor _asmy_pocchar)
    (if (not (Variables|/Game/Character/MyPOCChar.MyPOCChar_C|GetInvulnerable _asmy_pocchar))
      (bind _output_get (Variables|/Game/Character/MyPOCChar.MyPOCChar_C|SetCurrentHealth _asmy_pocchar (- (Variables|/Game/Character/MyPOCChar.MyPOCChar_C|GetCurrentHealth _asmy_pocchar) (Variables|Default|GetDamageAmount))))
      (Development|PrintString (Utilities|String|ToString(Integer) _output_get)))))

(event Custom|TagSearchBreak
  (Utilities|Array|ForEachLoopwithBreak (stale _outactors)) ; enters at Break
)

(event EventBeginPlay
  (Variables|Default|SetEngagementPhase 0)
  (Variables|Default|SetFirstEncounter true))

(event EventTick
  (params (DeltaSeconds :type Float%20%28single-precision%29))
  (Utilities|FlowControl|Sequence
    (:then_0
      (if (== (Variables|Default|GetEngagementPhase) 1)
        (Variables|Default|SetJumpingBack true)
        (Rendering|Components|TextRender|SetText (Variables|Default|GetSurprise) (Variables|Default|GetExclamationPoint))
        (else
          (Variables|Default|SetJumpingBack false)
          (Rendering|Components|TextRender|SetText (Variables|Default|GetSurprise) (Variables|Default|GetBlankSpace)))))
    (:then_1
      (if (<= (Variables|Default|GetEnemyHealth) 0)
        (Utilities|FlowControl|Delay 1.0)
        (Actor|DestroyActor)))
    (:then_2
      (if (Variables|Default|GetIsAttacking)
        _))))

(fn ConstructionScript
  (|CallParentFunction))