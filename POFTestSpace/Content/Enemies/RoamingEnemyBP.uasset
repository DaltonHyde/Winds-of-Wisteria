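; Roaming enemy Blueprint with sight sensing and a timed jump-back movement, left partly unwired.
; While JumpingBack is set, Tick adds input along the capsule's forward vector, scaled by JumpBackSpeed, then clears the flag after a delay.
; The see-pawn event is empty.
; Disconnected nodes hold the player chase, exclamation text and the only code setting JumpingBack true, so none of those run.
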(event `self.PawnSensing.OnSeePawn`
  (params (Pawn :type "Pawn Object Reference")))

(event `self.ReceiveTick`
  (params (DeltaSeconds :type "Float (single-precision)"))
  (if (`self.JumpingBack`)
    (`self.AddMovementInput` (`KismetMathLibrary.GetForwardVector` (`SceneComponent.K2_GetComponentRotation` (`self.CapsuleComponent`))) (`self.JumpBackSpeed`))
    (`KismetSystemLibrary.Delay` (`self.JumpBackPause`))
    (set `self.JumpingBack` false)))

(fn `UserConstructionScript`)